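; Player frog character Blueprint that adds visual effects, sprint input and skin display on top of its parent class.
; Direct sprint input starts and stops sprinting, and PlayHitEffect spawns a scaled-down super-jump particle at the mesh root.
; The skin RepNotify textures the hidden, owner-only first-person mesh through a dynamic material before calling parent logic.
; A first/third-person camera toggle exists but is disconnected, leaving the view-change input empty.
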(event `self.PlayHitEffect`
  (params (Index :type Integer))
  (`GameplayStatics.SpawnEmitterAtLocation` "/Game/Characters/FX_SuperJump.FX_SuperJump" (`SceneComponent.GetSocketLocation` (`self.Mesh`) "root") (struct) (0.5 0.5 0.5)))

(event `self.ReceiveBeginPlay`
  (bind _sm_frogoneview (`self.SM_FrogOneView`))
  (`PrimitiveComponent.SetOnlyOwnerSee` _sm_frogoneview true)
  (`SceneComponent.SetHiddenInGame` _sm_frogoneview true false))

(event `EnhancedInput|/Game/Characters/Input/IA_ChangeView`
  (params (ActionValue :type Boolean) (ElapsedSeconds :type "Float (double-precision)") (TriggeredSeconds :type "Float (double-precision)") (InputAction :type "InputAction Object Reference" :default "/Game/Characters/Input/IA_ChangeView.IA_ChangeView")))

(event `EnhancedInput|/Game/Characters/Input/IA_FrogDirectSprint`
  (params (ActionValue :type Boolean) (ElapsedSeconds :type "Float (double-precision)") (TriggeredSeconds :type "Float (double-precision)") (InputAction :type "InputAction Object Reference" :default "/Game/Characters/Input/IA_FrogDirectSprint.IA_FrogDirectSprint"))
  (:`Started`
    (`self.StartSprint`))
  (:`Completed`
    (`self.StopSprint`)))

(event `self.OnRep_SkinIndex`
  (bind _returnvalue (`PrimitiveComponent.CreateDynamicMaterialInstance` (`self.SM_FrogOneView`) 0 null "None"))
  (`MaterialInstanceDynamic.SetTextureParameterValue` _returnvalue "Skin" (`|GetArrayItem` (`self.SkinTextures`) (`self.SkinIndex`)))
  (`parent.OnRep_SkinIndex`))

(fn `UserConstructionScript`)