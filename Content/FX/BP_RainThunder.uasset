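; Weather actor that keeps a Niagara rain effect above the player and, while rain is enabled, fires lightning strikes at random intervals.
; Each strike moves the actor to a random spot ahead of the camera, yawed toward the player, and picks one of three bolt textures.
; A timeline animates the plane material's length and emissive alongside a thunder sound, then exposure compensation briefly changes on a post-process volume for a flash.
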(event `self.ReceiveBeginPlay`
  (bind _settings (`PostProcessVolume.Settings` (`self.PPvolume`)))
  (bind ((`AutoExposureMethod` _autoexposuremethod) (`ColorSaturation` _colorsaturation) (`ColorContrast` _colorcontrast) (`ColorOffsetShadows` _coloroffsetshadows) (`BloomIntensity` _bloomintensity) (`BloomThreshold` _bloomthreshold) (`DynamicGlobalIlluminationMethod` _dynamicglobalilluminationmethod) (`LumenRayLightingMode` _lumenraylightingmode) (`LumenSceneLightingQuality` _lumenscenelightingquality) (`LumenSceneDetail` _lumenscenedetail) (`LumenFinalGatherQuality` _lumenfinalgatherquality) (`ReflectionMethod` _reflectionmethod) (`LumenReflectionQuality` _lumenreflectionquality) (`AutoExposureBias` _autoexposurebias) (`AutoExposureMinBrightness` _autoexposureminbrightness) (`AutoExposureMaxBrightness` _autoexposuremaxbrightness) (`VignetteIntensity` _vignetteintensity) (`AmbientOcclusionIntensity` _ambientocclusionintensity) (`AmbientOcclusionRadius` _ambientocclusionradius) (`MotionBlurAmount` _motionbluramount) (`MotionBlurMax` _motionblurmax) (`MotionBlurTargetFPS` _motionblurtargetfps) (`MotionBlurPerObjectSize` _motionblurperobjectsize) (`WeightedBlendables` _weightedblendables)) (break `PostProcessSettings` _settings))
  (`SceneComponent.K2_DetachFromComponent` (`self.NS_Rain`) "KeepWorld" "KeepWorld" "KeepWorld" true)
  (`KismetSystemLibrary.Delay` (`KismetMathLibrary.RandomFloatInRange` 5.0 8.0) :!label _label)
  (if (`self.IsRain`)
    (`self.Strike`)
    (`KismetSystemLibrary.Delay` 0.2)
    (set `self.DefaultSettings` _settings)
    (set `PostProcessVolume.Settings` (make `PostProcessSettings` :`AutoExposureMethod` _autoexposuremethod :`ColorSaturation` _colorsaturation :`ColorContrast` _colorcontrast :`ColorOffsetShadows` _coloroffsetshadows :`BloomIntensity` _bloomintensity :`BloomThreshold` _bloomthreshold :`DynamicGlobalIlluminationMethod` _dynamicglobalilluminationmethod :`LumenRayLightingMode` _lumenraylightingmode :`LumenSceneLightingQuality` _lumenscenelightingquality :`LumenSceneDetail` _lumenscenedetail :`LumenFinalGatherQuality` _lumenfinalgatherquality :`ReflectionMethod` _reflectionmethod :`LumenReflectionQuality` _lumenreflectionquality :`AutoExposureBias` 5.0 :`AutoExposureMinBrightness` _autoexposureminbrightness :`AutoExposureMaxBrightness` _autoexposuremaxbrightness :`VignetteIntensity` _vignetteintensity :`AmbientOcclusionIntensity` _ambientocclusionintensity :`AmbientOcclusionRadius` _ambientocclusionradius :`MotionBlurAmount` _motionbluramount :`MotionBlurMax` _motionblurmax :`MotionBlurTargetFPS` _motionblurtargetfps :`MotionBlurPerObjectSize` _motionblurperobjectsize :`WeightedBlendables` _weightedblendables) (`self.PPvolume`))
    (`KismetSystemLibrary.Delay` 0.3)
    (set `PostProcessVolume.Settings` (`self.DefaultSettings`) (`self.PPvolume`))
    (goto _label)
    (else
      (goto _label))))

(event `self.ReceiveTick`
  (params (DeltaSeconds :type "Float (single-precision)"))
  (`SceneComponent.K2_SetWorldLocation` (`self.NS_Rain`) (+ (`self.K2_GetActorLocation` (`GameplayStatics.GetPlayerCharacter` 0)) (0.0 0.0 2000.0)) false false))

(event `Strike`
  (bind _thunder_plane (`self.Thunder_Plane`))
  (bind _returnvalue (`Controller.GetControlRotation` (`GameplayStatics.GetPlayerController` 0)))
  (bind _returnvalue_2 (`self.K2_GetActorLocation` (`GameplayStatics.GetPlayerCharacter` 0)))
  (bind _returnvalue_3 (+ (* (`KismetMathLibrary.GetForwardVector` _returnvalue) (`KismetMathLibrary.RandomFloatInRange` 5000.0 8000.0)) _returnvalue_2 (* (`KismetMathLibrary.GetRightVector` _returnvalue) (`KismetMathLibrary.RandomFloatInRange` -4000.0 4000.0)) (0.0 0.0 3000.0)))
  (bind (_returnvalue_roll _returnvalue_pitch _returnvalue_yaw) (`KismetMathLibrary.BreakRotator` (`KismetMathLibrary.FindLookAtRotation` _returnvalue_3 _returnvalue_2)))
  (`self.K2_SetActorLocationAndRotation` _returnvalue_3 (`KismetMathLibrary.MakeRotator` 0.0 0.0 _returnvalue_yaw))
  (`/Engine/EditorBlueprintResources/StandardMacros.IsValid` (`self.ThunderMaterial`)
    (:`Is Valid`
      _)
    (:`Is Not Valid`
      (bind _returnvalue_4 (`PrimitiveComponent.CreateDynamicMaterialInstance` (`self.Thunder_Plane`) 0 null "None"))
      (set `self.ThunderMaterial` _returnvalue_4)))
  (`MaterialInstanceDynamic.SetTextureParameterValue` (`self.ThunderMaterial`) "ThunderTexture" (select `int` (`KismetMathLibrary.RandomIntegerInRange` 0 2) :`0` "/Game/FX/IMage/Thunder.Thunder" :`1` "/Game/FX/IMage/Thunder2.Thunder2" :`2` "/Game/FX/IMage/Thunder3.Thunder3" :!type "Texture Object Reference"))
  (`GameplayStatics.PlaySound2D` "/Game/Sounds/Ques/SQ_Thunder.SQ_Thunder" 1.0 1.0 0.0 null null)
  (bind (_direction _length _thunder) (`Timeline|ThunderStrike` :!via `PlayFromStart`)
    (:`Update`
      (`MeshComponent.SetScalarParameterValueOnMaterials` _thunder_plane "Length" _length)
      (`MeshComponent.SetScalarParameterValueOnMaterials` _thunder_plane "Emissive" _thunder))))

(fn `SetRain`
  (params (Value :type Boolean))
  (`SceneComponent.SetHiddenInGame` (`self.NS_Rain`) (not Value) false)
  (set `self.IsRain` Value))

(fn `UserConstructionScript`)