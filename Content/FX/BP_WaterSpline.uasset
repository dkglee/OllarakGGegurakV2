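; BP_WaterSpline is an effect actor that runs a Niagara water system repeatedly along a spline.
; On BeginPlay it passes its drop rate and lifetime variables to the system's user parameters.
; Each Tick moves the effect to the current spline distance, then advances that distance by speed plus random jitter, without delta-time scaling.
; Past the spline's end, the distance resets to a small random offset from the start.
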(event `self.ReceiveBeginPlay`
  (bind _ns_waterspline (`self.NS_WaterSpline`))
  (`NiagaraComponent.SetVariableFloat` _ns_waterspline "User.DropRate" (`self.DropRate`))
  (`NiagaraComponent.SetVariableFloat` _ns_waterspline "User.LifeTime" (`self.LifeTime`)))

(event `self.ReceiveTick`
  (params (DeltaSeconds :type "Float (single-precision)"))
  (bind _returnvalue (`KismetMathLibrary.RandomFloatInRange` 0.0 20.0))
  (`SceneComponent.K2_SetWorldLocation` (`self.NS_WaterSpline`) (`SplineComponent.GetLocationAtDistanceAlongSpline` (`self.Spline`) (`self.Distance`) "World") false false)
  (bind _output_get (set `self.Distance` (+ (`self.Distance`) (`self.Speed`) _returnvalue)))
  (if (> _output_get (`SplineComponent.GetSplineLength` (`self.Spline`)))
    (set `self.Distance` _returnvalue)))

(fn `UserConstructionScript`)