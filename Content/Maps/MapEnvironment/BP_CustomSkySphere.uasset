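; BP_CustomSkySphere is a custom sky sphere Blueprint that derives sky colors by blending between dark and bright presets.
; SunZenithColor takes an alpha, stores it, and linearly interpolates the zenith, horizon, cloud and overall color variables from their dark and bright pairs.
; The event graph is inactive and the construction script only calls its parent, so nothing here calls the function or applies the colors to a material.
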(fn `SunZenithColor`
  (params (Alpha :type "Float (double-precision)"))
  (locals (DarkZenith :type "LinearColor Structure" :default (struct :`R` 0.01285 :`G` 0.027282 :`B` 0.085069 :`A` 1.0)) (BrightZenith :type "LinearColor Structure" :default (struct :`G` 0.275669 :`B` 0.956597 :`A` 1.0)) (DarkHorizon :type "LinearColor Structure" :default (struct :`R` 0.146882 :`G` 0.153594 :`B` 0.227431 :`A` 1.0)) (BrightHorizon :type "LinearColor Structure" :default (struct :`R` 0.622288 :`G` 0.650724 :`B` 0.963542 :`A` 1.0)) (AlphaValue :type "Float (double-precision)") (BrightCloud :type "LinearColor Structure" :default (struct :`R` 0.027798 :`G` 0.036823 :`B` 0.067708 :`A` 1.0)) (DarkCloud :type "LinearColor Structure" :default (struct :`R` 0.263013 :`G` 0.348404 :`B` 0.640625 :`A` 1.0)) (BrightOverall :type "LinearColor Structure" :default (struct :`R` 1.0 :`G` 1.0 :`B` 1.0 :`A` 1.0)) (DarkOverall :type "LinearColor Structure" :default (struct :`R` 0.605903 :`G` 0.605903 :`B` 0.605903 :`A` 1.0)))
  (set `local.AlphaValue` Alpha)
  (set `self.Zenith Color` (`KismetMathLibrary.LinearColorLerp` (`local.DarkZenith`) (`local.BrightZenith`) (`local.AlphaValue`)))
  (set `self.Horizon color` (`KismetMathLibrary.LinearColorLerp` (`local.DarkHorizon`) (`local.BrightHorizon`) (`local.AlphaValue`)))
  (set `self.Cloud color` (`KismetMathLibrary.LinearColorLerp` (`local.DarkCloud`) (`local.BrightCloud`) (`local.AlphaValue`)))
  (set `self.Overall Color` (`KismetMathLibrary.LinearColorLerp` (`local.DarkOverall`) (`local.BrightOverall`) (`local.AlphaValue`))))

(fn `UserConstructionScript`
  (`parent.UserConstructionScript`))