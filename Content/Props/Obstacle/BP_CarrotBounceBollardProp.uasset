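; Carrot bounce bollard obstacle prop that plays a squash-and-wobble animation when its hit effect fires.
; PlayHitEffect calls the parent effect, then runs a timeline that scales the pivot and tilts it in pitch and roll with a sine-based shake.
; A PlayHitEffect flag blocks the effect while set, and only the authority clears it when the timeline finishes.
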(event `self.PlayHitEffect`
  (params (Index :type Integer))
  (if (not (`self.bPlayHitEffect`))
    (`parent.PlayHitEffect` Index)
    (bind (_direction _carrotbouncebollardvec _carrotbouncebollardshake) (`Timeline|PlayHitEffectTimeline` :!via `PlayFromStart`)
      (:`Update`
        (`SceneComponent.SetWorldScale3D` (`self.PivotScene`) _carrotbouncebollardvec)
        (bind _returnvalue (* (`KismetMathLibrary.DegSin` _carrotbouncebollardshake) 4.0))
        (`SceneComponent.K2_SetRelativeRotation` (`self.PivotScene`) (`KismetMathLibrary.MakeRotator` _returnvalue _returnvalue) false false))
      (:`Finished`
        (if (`self.HasAuthority`)
          (set `self.bPlayHitEffect` false))))))

(fn `UserConstructionScript`)