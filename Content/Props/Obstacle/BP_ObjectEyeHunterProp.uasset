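; Eye Hunter obstacle prop that animates hit effects and shows a blur overlay from message display until mission end.
; Hit index 1 flattens the shield, then a timeline fans ten meshes upward and lifts both leaves outward.
; Other indices restore the shield, spin the meshes from random yaws to a shared random angle and pitch the leaves.
; A flag blocks overlapping effects; only the authority clears it when timelines finish.
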(event `self.ReceiveBeginPlay`
  (`parent.ReceiveBeginPlay`)
  (bind _returnvalue (`|CreateWidget` "/Game/UI/Obstacle/WBP_Blur.WBP_Blur_C"))
  (set `self.BlurUI` _returnvalue))

(event `self.PlayHitEffect`
  (params (Index :type Integer))
  (bind _returnvalue (`KismetMathLibrary.RandomFloatInRange` 360.0 1080.0))
  (if (not (`self.bPlayHitEffect`))
    (`parent.PlayHitEffect` Index)
    (set `self.RandRotValue` (`KismetMathLibrary.RandomFloatInRange` 360.0 720.0))
    (set `self.LeafArray` (`|MakeArray` (`self.left`) (`self.right`)))
    (set `self.MeshArray` (`|MakeArray` (`self.one`) (`self.two`) (`self.three`) (`self.four`) (`self.five`) (`self.six`) (`self.seven`) (`self.eight`) (`self.nine`) (`self.ten`)))
    (if (== Index 1)
      (`SceneComponent.SetRelativeScale3D` (`self.sm_shield`) (1.0 1.0 0.01))
      (for (_array_element _array_index) (`self.MeshArray`)
        (bind (_relativelocation_x _relativelocation_y _relativelocation_z) (`KismetMathLibrary.BreakVector` (`SceneComponent.RelativeLocation` _array_element)))
        (`KismetArrayLibrary.Array_Set` (`self.LocList`) _array_index _relativelocation_z))
      (bind (_direction _alpha _pitch) (`Timeline|Launch` :!via `PlayFromStart`)
        (:`Update`
          (`|ExecutionSequence`
            (:`then_0`
              (for (_array_element_2 _array_index_2) (`self.MeshArray`)
                (bind (_relativelocation_x_2 _relativelocation_y_2) (`KismetMathLibrary.BreakVector` (`SceneComponent.RelativeLocation` _array_element_2)))
                (bind _output (`|GetArrayItem` (`self.LocList`) _array_index_2))
                (`SceneComponent.K2_SetRelativeLocation` _array_element_2 (`KismetMathLibrary.MakeVector` _relativelocation_x_2 _relativelocation_y_2 (`KismetMathLibrary.Lerp` _output (+ _output (`KismetMathLibrary.Conv_IntToDouble` (* _array_index_2 10))) _alpha)) false false)))
            (:`then_1`
              (for (_array_element_3 _array_index_3) (`self.LeafArray`)
                (if (== _array_index_3 0)
                  (bind _relativelocation_x_3 (`KismetMathLibrary.BreakVector` (`SceneComponent.RelativeLocation` _array_element_3)))
                  (bind _returnvalue_2 (`KismetMathLibrary.Lerp` -104.0 10.0 _alpha))
                  (`SceneComponent.K2_SetRelativeLocation` _array_element_3 (`KismetMathLibrary.MakeVector` _relativelocation_x_3 (`KismetMathLibrary.Lerp` -13.0 -55.0 _alpha) _returnvalue_2) false false)
                  (else
                    (`SceneComponent.K2_SetRelativeLocation` _array_element_3 (`KismetMathLibrary.MakeVector` _relativelocation_x_3 (`KismetMathLibrary.Lerp` 13.0 55.0 _alpha) _returnvalue_2) false false)))
                (bind (_relativerotation_roll _relativerotation_pitch _relativerotation_yaw) (`KismetMathLibrary.BreakRotator` (`SceneComponent.RelativeRotation` _array_element_3)))
                (`SceneComponent.K2_SetRelativeRotation` _array_element_3 (`KismetMathLibrary.MakeRotator` _relativerotation_roll _pitch _relativerotation_yaw) false false)))))
        (:`Finished`
          (if (`self.HasAuthority`)
            (set `self.bPlayHitEffect` false))))
      (else
        (`SceneComponent.SetRelativeScale3D` (`self.sm_shield`) (1.0 1.0 1.0))
        (for (_array_element_4 _array_index_4) (`self.MeshArray`)
          (`KismetArrayLibrary.Array_Set` (`self.RotList`) _array_index_4 _returnvalue)
          (`SceneComponent.K2_SetRelativeRotation` _array_element_4 (`KismetMathLibrary.MakeRotator` 0.0 0.0 _returnvalue) false false))
        (bind (_direction_2 _rotatealpha _leafpitch) (`Timeline|TurnLeaf` :!via `PlayFromStart`)
          (:`Update`
            (`|ExecutionSequence`
              (:`then_0`
                (for (_array_element_5 _array_index_5) (`self.MeshArray`)
                  (`SceneComponent.K2_SetRelativeRotation` _array_element_5 (`KismetMathLibrary.MakeRotator` 0.0 0.0 (`KismetMathLibrary.Lerp` (`|GetArrayItem` (`self.RotList`) _array_index_5) (`self.RandRotValue`) _rotatealpha)) false false)))
              (:`then_1`
                (for _array_element_6 (`self.LeafArray`)
                  (bind (_relativerotation_roll_2 _relativerotation_pitch_2 _relativerotation_yaw_2) (`KismetMathLibrary.BreakRotator` (`SceneComponent.RelativeRotation` _array_element_6)))
                  (`SceneComponent.K2_SetRelativeRotation` _array_element_6 (`KismetMathLibrary.MakeRotator` _relativerotation_roll_2 _leafpitch _relativerotation_yaw_2) false false)))))
          (:`Finished`
            (if (`self.HasAuthority`)
              (set `self.bPlayHitEffect` false))))))))

(event `self.DisplayMessage`
  (bind _blurui (`self.BlurUI`))
  (`/Engine/EditorBlueprintResources/StandardMacros.IsValid` _blurui
    (:`Is Valid`
      (`UserWidget.AddToViewport` _blurui 0)
      (`parent.DisplayMessage`))))

(event `self.EndMission`
  (params (bIsSuccess :type Boolean))
  (bind _blurui (`self.BlurUI`))
  (`parent.EndMission` bIsSuccess)
  (`/Engine/EditorBlueprintResources/StandardMacros.IsValid` _blurui
    (:`Is Valid`
      (`Widget.RemoveFromParent` _blurui))))

(fn `UserConstructionScript`)