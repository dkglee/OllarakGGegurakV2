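; Pot cannon obstacle prop that animates a hit reaction and then fires a rolling ball.
; PlayHitEffect, when its flag is clear and the index is zero, runs a timeline that scales the mesh.
; When the timeline finishes, only the authority calls FireRollingBallAfterAnimation and clears the flag, so the shot waits for the animation.
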(event `self.PlayHitEffect`
  (params (Index :type Integer))
  (if (not (`self.bPlayHitEffect`))
    (if (== Index 0)
      (bind (_direction _hiteffectscale) (`Timeline|PlayHitEffectTimeline` :!via `PlayFromStart`)
        (:`Update`
          (`SceneComponent.SetRelativeScale3D` (`self.MeshComp`) _hiteffectscale))
        (:`Finished`
          (if (`self.HasAuthority`)
            (`RollingCannonProp.FireRollingBallAfterAnimation`)
            (set `self.bPlayHitEffect` false)))))))

(fn `UserConstructionScript`)