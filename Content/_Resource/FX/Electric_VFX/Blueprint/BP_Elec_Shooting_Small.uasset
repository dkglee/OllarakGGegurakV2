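; Electric VFX shooter that repeatedly fires a small projectile with a Niagara shooting effect.
; After a short delay on BeginPlay, it spawns a scaled-down ProjectileBP at its location, oriented by its Arrow component.
; Each shot also spawns NS_Elec_Shooting_Small at a fixed world-space offset and rotation, independent of the Arrow.
; NextArrow re-calls itself after a Delay to loop indefinitely; the random interval has equal bounds, so timing is constant.
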(event `NextArrow`
  (bind _returnvalue (`self.K2_GetActorLocation`))
  (bind (_returnvalue_location _returnvalue_rotation) (`KismetMathLibrary.BreakTransform` (`SceneComponent.K2_GetComponentToWorld` (`self.Arrow`))))
  (`|SpawnActorFromClass` (`self.ProjectileBP`) (`KismetMathLibrary.MakeTransform` _returnvalue _returnvalue_rotation (0.1 0.1 0.1)) "Undefined" "SelectDefaultAtRuntime" null null :!label _label)
  (`NiagaraFunctionLibrary.SpawnSystemAtLocation` "/Game/_Resource/FX/Electric_VFX/Niagara/Projectile/NS_Elec_Shooting_Small.NS_Elec_Shooting_Small" (+ _returnvalue (50.0 0.0 0.0)) (struct :`Pitch` 90.0 :`Roll` 90.0))
  (`KismetSystemLibrary.Delay` (`KismetMathLibrary.RandomFloatInRange` 3.0 3.0))
  (`self.NextArrow`))

(event `self.ReceiveBeginPlay`
  (`KismetSystemLibrary.Delay` 1.0)
  (goto _label))

(fn `UserConstructionScript`)